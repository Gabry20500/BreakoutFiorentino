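; Player Blueprint that slides its Body sideways and launches the ball, like a paddle.
; Move Right and Move Left axis inputs apply a swept local X offset, then zero the Body's physics velocity.
; BeginPlay caches the BP_Ball actor, and Space applies a fixed impulse to its Sphere through a DoOnce that is never reset, so the launch happens only once.
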(event EventBeginPlay
  (bind _returnvalue (Actor|GetActorOfClass "/Game/Ball/BP_Ball.BP_Ball_C"))
  (bind _asbp_ball (Utilities|Casting|CastToBP_Ball _returnvalue))
  (Variables|Default|SetBallRef _asbp_ball))

(event Input|AxisEvents|InputAxisMoveRight
  (params (AxisValue :type Float%20%28single-precision%29))
  (Transformation|AddLocalOffset (Variables|Default|GetBody) (Math|Vector|MakeVector (* AxisValue 12.0) 0.0 0.0) true false)
  (Physics|SetPhysicsLinearVelocity (Variables|Default|GetBody) "0, 0, 0" false "None"))

(event Input|AxisEvents|InputAxisMoveLeft
  (params (AxisValue :type Float%20%28single-precision%29))
  (Transformation|AddLocalOffset (Variables|Default|GetBody) (Math|Vector|MakeVector (* AxisValue 12.0) 0.0 0.0) true false)
  (Physics|SetPhysicsLinearVelocity (Variables|Default|GetBody) "0, 0, 0" false "None"))

(event Input|KeyboardEvents|SpaceBar
  (params (Key :type Key%20Structure :default "None"))
  (:Pressed
    (Utilities|FlowControl|DoOnce false
      (:Completed
        (Physics|AddImpulse (Variables|/Game/Ball/BP_Ball.BP_Ball_C|GetSphere (Variables|Default|GetBallRef)) "0,10000.000000,-28000.000000" "None" false)))))

(fn ConstructionScript)