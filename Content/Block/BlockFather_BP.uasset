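; BlockFather_BP is a block Blueprint, apparently a base class, that awards points and destroys itself when hit.
; BeginPlay finds and caches references to BP_Player and BP_Ball, though the ball reference is not used afterward.
; Any overlap with its Box component, without filtering the other actor, adds Point to the player's Score, then destroys the block after a brief delay.
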(event OnComponentBeginOverlap(Box)
  (params (OverlappedComponent :type Primitive%20Component%20Object%20Reference) (OtherActor :type Actor%20Object%20Reference) (OtherComp :type Primitive%20Component%20Object%20Reference) (OtherBodyIndex :type Integer) (bFromSweep :type Boolean) (SweepResult :type Hit%20Result%20Structure%20%28by%20ref%29))
  (bind _playerref (Variables|Default|GetPlayerRef))
  (Variables|/Game/Player/BP_Player.BP_Player_C|SetScore _playerref (+ (Variables|/Game/Player/BP_Player.BP_Player_C|GetScore _playerref) (Variables|Default|GetPoint)))
  (Utilities|FlowControl|Delay 0.05)
  (Actor|DestroyActor))

(event EventBeginPlay
  ;[1 1 1] player ref
  (bind _returnvalue (Actor|GetActorOfClass "/Game/Player/BP_Player.BP_Player_C"))
  (bind _asbp_player (Utilities|Casting|CastToBP_Player _returnvalue))
  (Variables|Default|SetPlayerRef _asbp_player)
  ;[1 1 1] Ball ref
  (bind _returnvalue_2 (Actor|GetActorOfClass "/Game/Ball/BP_Ball.BP_Ball_C"))
  (bind _asbp_ball (Utilities|Casting|CastToBP_Ball _returnvalue_2))
  (Variables|Default|SetBallRef _asbp_ball))

(event Collision|EventActorBeginOverlap
  (params (OtherActor :type Actor%20Object%20Reference)))

(event EventTick
  (params (DeltaSeconds :type Float%20%28single-precision%29)))

(fn ConstructionScript)